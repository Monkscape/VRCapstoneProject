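; Wind turbine actor that triggers a petal wind simulation on flowers entering its WindRadius component.
; On begin overlap it prints the other actor, then class-checks and casts it to Flower before calling SimulatePetalWind.
; End overlap only clears an InWindRadius flag, which nothing here sets or reads.
; A LaunchSphere branch that would call LaunchBall is disconnected and never runs.
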(event `self.WindRadius.OnComponentBeginOverlap`
  (params (OverlappedComponent :type "PrimitiveComponent Object Reference") (OtherActor :type "Actor Object Reference") (OtherComp :type "PrimitiveComponent Object Reference") (OtherBodyIndex :type Integer) (bFromSweep :type Boolean) (SweepResult :type "HitResult Structure (by ref)"))
  (`KismetSystemLibrary.PrintString` (`KismetStringLibrary.Conv_ObjectToString` OtherActor))
  (if (`KismetMathLibrary.ClassIsChildOf` (`GameplayStatics.GetObjectClass` OtherActor) "/Game/Blueprints/Flower.Flower_C")
    (bind _asflower (cast `/Game/Blueprints/Flower` OtherActor))
    (`/Game/Blueprints/Flower.SimulatePetalWind` _asflower)))

(event `self.WindRadius.OnComponentEndOverlap`
  (params (OverlappedComponent :type "PrimitiveComponent Object Reference") (OtherActor :type "Actor Object Reference") (OtherComp :type "PrimitiveComponent Object Reference") (OtherBodyIndex :type Integer))
  (set `self.InWindRadius` false))

(fn `UserConstructionScript`)