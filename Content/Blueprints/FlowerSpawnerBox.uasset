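; FlowerSpawnerBox scatters Flower actors at random spots within a box area when play begins.
; BeginPlay loops over NumberOfFlowers, calling FindLocation for each spawn and adjusting for collisions while always spawning.
; FindLocation picks a random X and Y within the FlowerSpawnBounds component's bounds and fixes Z at world zero, ignoring the box's height.
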(event `self.ReceiveBeginPlay`
  (for _ (range (+ (`self.NumberOfFlowers`) 1))
    (bind _returnvalue (`self.FindLocation`))
    (`|SpawnActorFromClass` "/Game/Blueprints/Flower.Flower_C" _returnvalue "AdjustIfPossibleButAlwaysSpawn" "OverrideRootScale" null null)))

(fn `FindLocation`
  (returns (ReturnValue :type "Transform Structure"))
  (bind (_origin _boxextent) (`KismetSystemLibrary.GetComponentBounds` (`self.FlowerSpawnBounds`)))
  (bind _x (.x _origin))
  (bind _y (.y _origin))
  (bind _x_2 (.x _boxextent))
  (bind _y_2 (.y _boxextent))
  (return (`KismetMathLibrary.Conv_VectorToTransform` (`KismetMathLibrary.MakeVector` (`KismetMathLibrary.RandomFloatInRange` (- _x _x_2) (+ _x _x_2)) (`KismetMathLibrary.RandomFloatInRange` (- _y _y_2) (+ _y _y_2))))))

(fn `UserConstructionScript`)