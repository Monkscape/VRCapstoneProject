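; Sphere shape actor that reacts when something begins overlapping its static mesh.
; Each overlap gathers every Flower actor in the level and calls MoveFlower on it.
; Within that same loop, it swaps its own material to gold if CurrentLandscape overlaps the sphere, otherwise to the basic floor material.
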(event `self.StaticMesh.OnComponentBeginOverlap`
  (params (OverlappedComponent :type "PrimitiveComponent Object Reference") (OtherActor :type "Actor Object Reference") (OtherComp :type "PrimitiveComponent Object Reference") (OtherBodyIndex :type Integer) (bFromSweep :type Boolean) (SweepResult :type "HitResult Structure (by ref)"))
  (bind _outactors (`GameplayStatics.GetAllActorsOfClass` "/Game/Blueprints/Flower.Flower_C"))
  (for _array_element _outactors
    (`/Game/Blueprints/Flower.Move Flower` _array_element)
    (if (`self.IsOverlappingActor` (`self.Current Landscape`) self)
      (`PrimitiveComponent.SetMaterial` (`self.StaticMesh`) 0 "/Game/StarterContent/Materials/M_Metal_Gold.M_Metal_Gold")
      (else
        (`PrimitiveComponent.SetMaterial` (`self.StaticMesh`) 0 "/Game/StarterContent/Materials/M_Basic_Floor.M_Basic_Floor")))))

(fn `UserConstructionScript`)