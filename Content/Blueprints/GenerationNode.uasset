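; Level generation actor that builds a landscape, scatters flowers and wind turbines, then spawns and possesses a motion controller pawn.
; On BeginPlay, a seeded or random stream feeds the LandscapeGenerator, flower count, flower seeds and random placements.
; Flowers and turbines spawn at maximum terrain height and step downward until they overlap the landscape.
; GenerationType shapes the landscape call and picks turbine facing and the player spawn point.
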(event `self.ReceiveBeginPlay`
  (bind _returnvalue (`KismetMathLibrary.RandomInteger` 2147483647))
  (`self.VerifyFlowerRange`)
  (switch `/Game/Blueprints/LandscapeType` (`self.Generation Type`)
    (:`NewEnumerator0`
      (set `self.TurbineAngle` 90.0 :!label _label))
    (:`NewEnumerator1`
      (goto _label))
    (:`NewEnumerator2`
      (goto _label))
    (:`NewEnumerator3`
      (set `self.TurbineAngle` 270.0))
    (:`NewEnumerator5`
      (goto _label))
    (:`NewEnumerator6`
      (goto _label)))
  (if (`self.UseSeed`)
    (set `self.RandomStream` (`KismetMathLibrary.MakeRandomStream` (`self.Seed Value`)))
    (else
      (set `self.RandomStream` (`KismetMathLibrary.MakeRandomStream` _returnvalue))
      (set `self.Seed Value` _returnvalue)))
  (bind _returnvalue_2 (`|SpawnActorFromClass` "/Game/Blueprints/LandscapeGenerator.LandscapeGenerator_C" (`KismetMathLibrary.MakeTransform` (`self.CenterLandscape`)) "Undefined" "OverrideRootScale" null (`self.Max Height`) (`self.Generation Type`) (`self.RandomStream`) (`self.Grid Size`) null))
  (set `self.Landscape` _returnvalue_2)
  (for _ (range 1 (+ (`KismetMathLibrary.RandomIntegerInRangeFromStream` (`self.Min Flowers`) (`self.Max Flowers`) (`self.RandomStream`)) 1))
    (bind _max_height (`/Game/Blueprints/LandscapeGenerator.Get Maximum Height` (`self.Landscape`)))
    (bind _returnvalue_3 (`|SpawnActorFromClass` "/Game/Blueprints/Flower.Flower_C" (`self.GenerateRandomFlowerLocation` _max_height) "Undefined" "OverrideRootScale" null (`KismetMathLibrary.RandomIntegerFromStream` 1000000 (`self.RandomStream`)) null))
    (`self.MoveActorToLandscape` _returnvalue_3))
  (for _ (range 1 (+ (`self.NumberOfTurbines`) 1))
    (bind _returnvalue_4 (`|SpawnActorFromClass` "/Game/Blueprints/WindTurbine.WindTurbine_C" (`self.GenerateRandomTurbineLocation` _max_height (`self.TurbineAngle`)) "Undefined" "OverrideRootScale" null null))
    (`self.MoveActorToLandscape` _returnvalue_4)
    (`self.K2_AddActorLocalOffset` _returnvalue_4 (0.0 0.0 -2.0) false false))
  (bind _player_spawn_point (`self.GeneratePlayerSpawnPoint`))
  (bind _returnvalue_5 (`|SpawnActorFromClass` "/Game/VirtualRealityBP/Blueprints/MotionControllerPawn.MotionControllerPawn_C" _player_spawn_point "Undefined" "OverrideRootScale" null null))
  (`Controller.Possess` (`GameplayStatics.GetPlayerController` 0) _returnvalue_5))

(fn `GeneratePlayerSpawnPoint`
  (returns (`Player Spawn Point` :type "Transform Structure"))
  (locals (`Landscape Location` :type "Vector Structure") (`Spawn Point` :type "Transform Structure") (`Starting Height` :type "Float (double-precision)" :default 50.0))
  (bind _starting_height (`local.Starting Height`))
  (bind _returnvalue (+ (.x (`local.Landscape Location`)) 25.0))
  (set `local.Landscape Location` (`self.K2_GetActorLocation` (`self.Landscape`)))
  (switch `/Game/Blueprints/LandscapeType` (`self.Generation Type`)
    (:`NewEnumerator0`
      (set `local.Spawn Point` (`KismetMathLibrary.MakeTransform` (`KismetMathLibrary.MakeVector` 0.0 0.0 (`local.Starting Height`))) :!label _label))
    (:`NewEnumerator1`
      (goto _label))
    (:`NewEnumerator2`
      (set `local.Spawn Point` (`KismetMathLibrary.MakeTransform` (`KismetMathLibrary.MakeVector` _returnvalue 0.0 _starting_height))))
    (:`NewEnumerator3`
      (bind _max_height (`/Game/Blueprints/LandscapeGenerator.Get Maximum Height` (`self.Landscape`)))
      (set `local.Spawn Point` (`KismetMathLibrary.MakeTransform` (`KismetMathLibrary.MakeVector` _returnvalue 0.0 (+ _max_height _starting_height)))))
    (:`NewEnumerator5`
      (goto _label))
    (:`NewEnumerator6`
      (goto _label)))
  (return (`local.Spawn Point`)))

(fn `MoveActorToLandscape`
  (params (Actor :type "Actor Object Reference"))
  (locals (`Number of Loops` :type Integer))
  (bind _max_height (`/Game/Blueprints/LandscapeGenerator.Get Maximum Height` (`self.Landscape`)))
  (while (!= (`self.IsOverlappingActor` Actor (`self.Landscape`)) true)
    (`/Engine/EditorBlueprintResources/StandardMacros.IncrementInt` (`local.Number of Loops`)
      (:`  `
        (`self.K2_AddActorLocalOffset` Actor (`KismetMathLibrary.MakeVector` 0.0 0.0 (* (+ (/ _max_height 1000.0) 1.0) -1.0)) false false))))
  (`KismetSystemLibrary.PrintString` (`KismetStringLibrary.Conv_IntToString` (`local.Number of Loops`))))

(fn `UserConstructionScript`)

(fn `VerifyFlowerRange`
  (locals (Temp :type Integer))
  (bind _min_flowers (`self.Min Flowers`))
  (bind _max_flowers (`self.Max Flowers`))
  (if (not (<= _min_flowers _max_flowers))
    (bind _output_get (set `local.Temp` _min_flowers))
    (set `self.Min Flowers` _max_flowers)
    (set `self.Max Flowers` _output_get)))