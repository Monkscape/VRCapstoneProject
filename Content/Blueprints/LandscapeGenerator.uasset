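; LandscapeGenerator builds a flat, grid-based procedural mesh in its construction script, sized by GridSize.
; It lays out corner vertices at 100-unit spacing, then appends a center vertex for each cell.
; AddTriangle fills the index list with two triangles per cell, joining two opposite edges to the center and leaving the other two sides unfilled.
; The vertex and index arrays then feed CreateMeshSectionLinearColor on the ProceduralMesh.
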(fn `Add Triangle`
  (params (Vertice1 :type Integer) (Vertice2 :type Integer) (Vertice3 :type Integer))
  (bind _triangles (`self.Triangles`))
  (`KismetArrayLibrary.Array_Add` _triangles Vertice1)
  (`KismetArrayLibrary.Array_Add` _triangles Vertice2)
  (`KismetArrayLibrary.Array_Add` _triangles Vertice3))

(fn `UserConstructionScript`
  (locals (offset_y :type "Float (double-precision)") (offset_x :type "Float (double-precision)") (vert_pos1 :type Integer) (vert_pos2 :type Integer :default 1) (vert_pos3 :type Integer))
  (bind _grid_size (`self.Grid Size`))
  (bind _grid_size_2 (`self.Grid Size`))
  (bind _returnvalue (+ (`self.Grid Size`) 1))
  (bind _returnvalue_2 (+ (`self.Grid Size`) 1))
  (bind _returnvalue_3 (+ (`self.Grid Size`) 1))
  (for _index (range 1 (+ (* _returnvalue_2 _returnvalue_2) 1))
    (`KismetArrayLibrary.Array_Add` (`self.Vertices`) (`KismetMathLibrary.MakeVector` (`local.offset_x`) (`local.offset_y`)))
    (set `local.offset_y` (+ (`local.offset_y`) 100.0))
    (if (== (mod _index (+ (`self.Grid Size`) 1)) 0)
      (set `local.offset_x` (+ (`local.offset_x`) 100.0))
      (set `local.offset_y` 0.0)))
  (`KismetSystemLibrary.PrintString` "Adding Centerpoints")
  (set `local.offset_x` 50.0)
  (set `local.offset_y` 50.0)
  (for _index_2 (range 1 (+ (* _grid_size _grid_size) 1))
    (`KismetArrayLibrary.Array_Add` (`self.Vertices`) (`KismetMathLibrary.MakeVector` (`local.offset_x`) (`local.offset_y`)))
    (set `local.offset_y` (+ (`local.offset_y`) 100.0))
    (if (== (mod _index_2 (`self.Grid Size`)) 0)
      (set `local.offset_x` (+ (`local.offset_x`) 100.0))
      (set `local.offset_y` 50.0)))
  (set `local.vert_pos3` (* _returnvalue _returnvalue))
  (for _index_3 (range 1 (+ (* _grid_size_2 _grid_size_2) 1))
    (`self.Add Triangle` (`local.vert_pos1`) (`local.vert_pos2`) (`local.vert_pos3`))
    (`self.Add Triangle` (+ (`local.vert_pos1`) _returnvalue_3) (+ (`local.vert_pos2`) _returnvalue_3) (`local.vert_pos3`))
    (if (== (mod _index_3 (`self.Grid Size`)) 0)
      (set `local.vert_pos1` (+ (`local.vert_pos1`) 2))
      (set `local.vert_pos2` (+ (`local.vert_pos2`) 2))
      (else
        (`/Engine/EditorBlueprintResources/StandardMacros.IncrementInt` (`local.vert_pos1`)
          (:`  `
            (`/Engine/EditorBlueprintResources/StandardMacros.IncrementInt` (`local.vert_pos2`)
              (:`  `
                _))))))
    (`/Engine/EditorBlueprintResources/StandardMacros.IncrementInt` (`local.vert_pos3`)))
  (`ProceduralMeshComponent.CreateMeshSection_LinearColor` :`self` (`self.ProceduralMesh`) :`Vertices` (`self.Vertices`) :`Triangles` (`self.Triangles`)))