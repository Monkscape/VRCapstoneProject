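; Procedural flower actor that can be picked up, dropped and shed its petals in a simulated wind.
; The construction script uses a seeded stream to vary stem height and petal count, size and angle, spawning petal meshes in a ring with dynamic materials.
; BeginPlay applies two petal colors to those materials.
; Pickup attaches the flower, Drop detaches it with physics on all parts, and wind pushes physics-enabled petals sideways.
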(event `Event SimulatePetalWind`
  ;[1 1 1] Event Simulate Petal Wind
  (for _array_element (`self.Petals`)
    (`PrimitiveComponent.SetCollisionEnabled` _array_element "PhysicsOnly")
    (`PrimitiveComponent.SetSimulatePhysics` _array_element true)
    (`PrimitiveComponent.AddForce` _array_element (0.0 100.0 0.0) "None" false)))

(event `/Game/VirtualRealityBP/Blueprints/PickupActorInterface.Pickup`
  (params (AttachTo :type "SceneComponent Object Reference"))
  ;[1 1 1] Event Pickup
  (`PrimitiveComponent.SetSimulatePhysics` (`self.Stem`) false)
  (`SceneComponent.K2_AttachToComponent` (`self.K2_GetRootComponent`) AttachTo "None" "KeepWorld" "KeepWorld" "KeepWorld" false))

(event `/Game/VirtualRealityBP/Blueprints/PickupActorInterface.Drop`
  ;[1 1 1] Event Drop
  (`PrimitiveComponent.SetSimulatePhysics` (`self.Stem`) true)
  (`PrimitiveComponent.SetSimulatePhysics` (`self.Stamen`) true)
  (for _array_element (`self.Petals`)
    (`PrimitiveComponent.SetCollisionEnabled` _array_element "PhysicsOnly")
    (`PrimitiveComponent.SetSimulatePhysics` _array_element true))
  (`self.K2_DetachFromActor` "KeepWorld" "KeepWorld" "KeepWorld"))

(event `self.ReceiveBeginPlay`
  ;[1 1 1] Event Begin Play
  (for _array_element (`self.Petal Material`)
    (`MaterialInstanceDynamic.SetVectorParameterValue` _array_element "Color1" (`self.PetalColor`))
    (`MaterialInstanceDynamic.SetVectorParameterValue` _array_element "Color2" (`self.PetalColor2`))))

(fn `UserConstructionScript`
  (locals (`Pivot Point` :type "Float (double-precision)" :default 0.0) (`Petal Size` :type "Float (double-precision)") (`Petal Length` :type "Float (double-precision)") (`Petal Offset` :type "Float (double-precision)"))
  (bind _petal_size (`local.Petal Size`))
  (bind _petal_length (`local.Petal Length`))
  (bind _returnvalue (+ (`local.Petal Length`) 0.5))
  (bind _returnvalue_2 (`KismetMathLibrary.MakeVector` 0.0 2.5 (* (.z (`SceneComponent.K2_GetComponentScale` (`self.Stem`))) 100.0)))
  (set `self.RandomStream` (`KismetMathLibrary.MakeRandomStream` (`self.Seed Value`)))
  (set `local.Petal Size` (`KismetMathLibrary.RandomFloatInRangeFromStream` 0.01 0.03 (`self.RandomStream`)))
  (set `local.Petal Length` (`KismetMathLibrary.RandomFloatInRangeFromStream` 0.1 0.2 (`self.RandomStream`)))
  (set `local.Petal Offset` (`KismetMathLibrary.RandomFloatInRangeFromStream` -30.0 30.0 (`self.RandomStream`)))
  (set `self.NumberOfPetals` (`KismetMathLibrary.RandomIntegerInRangeFromStream` 5 20 (`self.RandomStream`)))
  (set `self.PetalColor` (`self.PickRandomColor`))
  (set `self.PetalColor2` (`self.PickRandomColor`))
  (`SceneComponent.SetWorldScale3D` (`self.Stem`) (`KismetMathLibrary.MakeVector` (.x (`SceneComponent.K2_GetComponentScale` (`self.Stem`))) (.y (`SceneComponent.K2_GetComponentScale` (`self.Stem`))) (`KismetMathLibrary.RandomFloatInRangeFromStream` 0.25 0.3 (`self.RandomStream`))))
  (`SceneComponent.K2_SetRelativeTransform` (`self.Bounds`) (`KismetMathLibrary.MakeTransform` (`KismetMathLibrary.MakeVector` 0.0 0.0 (+ (/ (* _returnvalue 65.0) 2.0) 2.5)) (struct) (`KismetMathLibrary.MakeVector` _petal_length _petal_length _returnvalue)) false false)
  (`SceneComponent.K2_SetRelativeLocation` (`self.Stamen`) _returnvalue_2 false false)
  (set `local.Pivot Point` (/ 360.0 (`KismetMathLibrary.Conv_IntToDouble` (`self.NumberOfPetals`))))
  (for _index (range 1 (+ (`self.NumberOfPetals`) 1))
    (bind _returnvalue_3 (`AddComponent|NODE_AddStaticMeshComponent-2` :`RelativeTransform` (`KismetMathLibrary.MakeTransform` (`KismetMathLibrary.MakeVector` (.x _returnvalue_2) (.y _returnvalue_2) (+ (.z _returnvalue_2) 5.0)) (`KismetMathLibrary.MakeRotator` 0.0 (+ (* (`KismetMathLibrary.Conv_IntToDouble` _index) (`local.Pivot Point`)) (`local.Petal Offset`))) (`KismetMathLibrary.MakeVector` _petal_size _petal_size (`local.Petal Length`)))))
    (bind _returnvalue_4 (`PrimitiveComponent.CreateDynamicMaterialInstance` _returnvalue_3 0 "/Game/Materials/PetalColor.PetalColor" "None"))
    (`KismetArrayLibrary.Array_Add` (`self.Petal Material`) _returnvalue_4)
    (`KismetArrayLibrary.Array_Add` (`self.Petals`) _returnvalue_3)))