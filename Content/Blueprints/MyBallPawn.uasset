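; MyBallPawn is a ball pawn Blueprint that takes on a random color when play begins.
; The construction script sets StaticMesh to a sphere, stores a dynamic material instance created from it, and passes that instance to the Cube component as its source material.
; BeginPlay then sets the stored material's Color parameter from random red, green and blue values.
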(event `self.ReceiveBeginPlay`
  (`MaterialInstanceDynamic.SetVectorParameterValue` (`self.Dynamic Material`) "Color" (`KismetMathLibrary.MakeColor` (`KismetMathLibrary.RandomFloatInRange` 0.0 1.0) (`KismetMathLibrary.RandomFloatInRange` 0.0 1.0) (`KismetMathLibrary.RandomFloatInRange` 0.0 1.0))))

(fn `UserConstructionScript`
  (bind _staticmesh (`self.StaticMesh`))
  (`StaticMeshComponent.SetStaticMesh` _staticmesh "/Game/StarterContent/Shapes/Shape_Sphere.Shape_Sphere")
  (bind _returnvalue (`PrimitiveComponent.CreateDynamicMaterialInstance` _staticmesh 0 null "None"))
  (set `self.Dynamic Material` _returnvalue)
  (`PrimitiveComponent.CreateDynamicMaterialInstance` (`self.Cube`) 0 (`self.Dynamic Material`) "None"))