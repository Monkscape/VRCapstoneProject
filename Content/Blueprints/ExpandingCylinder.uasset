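; ExpandingCylinder is an actor whose static mesh continually grows and shrinks along its Z scale between MinHeight and MaxHeight.
; Construction sets CylinderHeight to 1, then each Tick steps it one unit by the Ascending flag and ChangeCylinderHeight applies it as world scale, preserving X and Y.
; Ascending flips only on exact equality with a limit, and the per-frame step ignores delta time, so speed follows frame rate.
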(event `self.ReceiveTick`
  (params (DeltaSeconds :type "Float (single-precision)"))
  (if (`self.Ascending`)
    (set `self.CylinderHeight` (+ (`self.CylinderHeight`) 1.0))
    (else
      (set `self.CylinderHeight` (- (`self.CylinderHeight`) 1.0))))
  (`self.ChangeCylinderHeight`)
  (if (`self.Ascending`)
    (`/Engine/EditorBlueprintResources/StandardMacros.CompareFloat` (`self.CylinderHeight`) (`self.MaxHeight`)
      (:`==`
        (set `self.Ascending` false)))
    (else
      (`/Engine/EditorBlueprintResources/StandardMacros.CompareFloat` (`self.CylinderHeight`) (`self.MinHeight`)
        (:`==`
          (set `self.Ascending` true))))))

(fn `ChangeCylinderHeight`
  (`SceneComponent.SetWorldScale3D` (`self.StaticMesh`) (`KismetMathLibrary.MakeVector` (.x (`SceneComponent.K2_GetComponentScale` (`self.StaticMesh`))) (.y (`SceneComponent.K2_GetComponentScale` (`self.StaticMesh`))) (`self.CylinderHeight`))))

(fn `UserConstructionScript`
  (set `self.CylinderHeight` 1.0))